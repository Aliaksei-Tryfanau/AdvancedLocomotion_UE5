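; Player character Blueprint that handles Enhanced Input movement, look, weapon switching and aiming.
; Weapon switching sets the equipped gun and links the matching unarmed, pistol or rifle animation class layers.
; Aim press and release switch the movement gate (gait) through UpdateGate, which applies that gate's speed, acceleration and braking settings from a map.
; Gun and gate changes are both sent to the mesh's anim instance as messages.
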(event `self.ReceiveBeginPlay`
  (bind _asplayer_controller (cast `PlayerController` (`self.GetController`)))
  (`EnhancedInputSubsystemInterface.AddMappingContext` (pcsubsystem `EnhancedInputLocalPlayerSubsystem` _asplayer_controller) "/Game/ALS/Input/IMC_PlayerCharacter.IMC_PlayerCharacter" 0 (struct))
  (`SkeletalMeshComponent.LinkAnimClassLayers` (`self.Mesh`) "/Game/ALS/Animation/ABP_Unarmed.ABP_Unarmed_C")
  (`self.UpdateGate` "NewEnumerator1"))

(event `EnhancedInput|/Game/ALS/Input/Actions/IA_SwitchWeapon`
  (params (ActionValue :type "Float (double-precision)") (ElapsedSeconds :type "Float (double-precision)") (TriggeredSeconds :type "Float (double-precision)") (InputAction :type "InputAction Object Reference" :default "/Game/ALS/Input/Actions/IA_SwitchWeapon.IA_SwitchWeapon"))
  (bind _mesh (`self.Mesh`))
  ;[1 1 1] Inputs
  (:`Started`
    (switch `int` (`KismetMathLibrary.FTrunc` ActionValue)
      (:`0`
        (set `self.EquippedGun` "NewEnumerator0" :!label _label)
        (`SkeletalMeshComponent.LinkAnimClassLayers` _mesh "/Game/ALS/Animation/ABP_Unarmed.ABP_Unarmed_C"))
      (:`1`
        (goto _label))
      (:`2`
        (set `self.EquippedGun` "NewEnumerator1")
        (`SkeletalMeshComponent.LinkAnimClassLayers` _mesh "/Game/ALS/Animation/ABP_Pistol.ABP_Pistol_C"))
      (:`3`
        (set `self.EquippedGun` "NewEnumerator2")
        (`SkeletalMeshComponent.LinkAnimClassLayers` _mesh "/Game/ALS/Animation/ABP_Rifle.ABP_Rifle_C")))
    (message `/Game/ALS/Interfaces/BPI_AnimationInterface.ReceiveEquippedGun` (`SkeletalMeshComponent.GetAnimInstance` _mesh) (`self.EquippedGun`))))

(event `EnhancedInput|/Game/ALS/Input/Actions/IA_Look`
  (params (ActionValue :type "Vector2D Structure") (ElapsedSeconds :type "Float (double-precision)") (TriggeredSeconds :type "Float (double-precision)") (InputAction :type "InputAction Object Reference" :default "/Game/ALS/Input/Actions/IA_Look.IA_Look"))
  (bind (_x _y) (`KismetMathLibrary.BreakVector2D` ActionValue))
  ;[1 1 1] Inputs
  (:`Triggered`
    (`self.AddControllerYawInput` _x)
    (`self.AddControllerPitchInput` _y)))

(event `EnhancedInput|/Game/ALS/Input/Actions/IA_Move`
  (params (ActionValue :type "Vector2D Structure") (ElapsedSeconds :type "Float (double-precision)") (TriggeredSeconds :type "Float (double-precision)") (InputAction :type "InputAction Object Reference" :default "/Game/ALS/Input/Actions/IA_Move.IA_Move"))
  (bind (_x _y) (`KismetMathLibrary.BreakVector2D` ActionValue))
  (bind (_returnvalue_roll _returnvalue_pitch _returnvalue_yaw) (`KismetMathLibrary.BreakRotator` (`self.GetControlRotation`)))
  (bind (_returnvalue_roll_2 _returnvalue_pitch_2 _returnvalue_yaw_2) (`KismetMathLibrary.BreakRotator` (`self.GetControlRotation`)))
  ;[1 1 1] Inputs
  (:`Triggered`
    (`self.AddMovementInput` (`KismetMathLibrary.GetRightVector` (`KismetMathLibrary.MakeRotator` _returnvalue_roll 0.0 _returnvalue_yaw)) _x)
    (`self.AddMovementInput` (`KismetMathLibrary.GetForwardVector` (`KismetMathLibrary.MakeRotator` 0.0 0.0 _returnvalue_yaw_2)) _y)))

(event `EnhancedInput|/Game/ALS/Input/Actions/IA_Aim`
  (params (ActionValue :type Boolean) (ElapsedSeconds :type "Float (double-precision)") (TriggeredSeconds :type "Float (double-precision)") (InputAction :type "InputAction Object Reference" :default "/Game/ALS/Input/Actions/IA_Aim.IA_Aim"))
  ;[1 1 1] Inputs
  (:`Started`
    (`self.UpdateGate` "NewEnumerator0"))
  (:`Completed`
    (`self.UpdateGate` "NewEnumerator1")))

(fn `UpdateGate`
  (params (Gate :type "/Game/ALS/Enums/E_Gate Enum" :default "NewEnumerator0"))
  (bind _charactermovement (`self.CharacterMovement`))
  (bind _output_get (set `self.CurrentGate` Gate))
  (message `/Game/ALS/Interfaces/BPI_AnimationInterface.ReceiveCurrentGate` (`SkeletalMeshComponent.GetAnimInstance` (`self.Mesh`)) _output_get)
  (`|ExecutionSequence`
    (:`then_0`
      (bind (_maxwalkspeed _maxacceleration _breakingdeceleration _breakingfrictionfactor _breakingfriction _useseparatebreakingfriction) (break `/Game/ALS/Structs/S_GateSettings` (`BlueprintMapLibrary.Map_Find` (`self.GateSettings`) _output_get)))
      (set `CharacterMovementComponent.MaxWalkSpeed` _maxwalkspeed _charactermovement))
    (:`then_1`
      (set `CharacterMovementComponent.MaxAcceleration` _maxacceleration _charactermovement))
    (:`then_2`
      (set `CharacterMovementComponent.BrakingDecelerationWalking` _breakingdeceleration _charactermovement))
    (:`then_3`
      (set `CharacterMovementComponent.BrakingFrictionFactor` _breakingfrictionfactor _charactermovement))
    (:`then_4`
      (set `CharacterMovementComponent.BrakingFriction` _breakingfriction _charactermovement))
    (:`then_5`
      (set `CharacterMovementComponent.bUseSeparateBrakingFriction` _useseparatebreakingfriction _charactermovement))))

(fn `UserConstructionScript`)